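; BP_Floor is a floor actor that slides its static mesh vertically while its play and move-up flags are set.
; Tick offsets the mesh's relative Z by negated speed scaled by delta time, clearing the move-up flag once Z reaches an upper limit.
; An X-axis movement branch that would re-enable the flag is disconnected, and MoveDown is an empty stub.
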(event `self.ReceiveTick`
  (params (DeltaSeconds :type "Float (single-precision)"))
  (bind _staticmesh (`self.StaticMesh`))
  (bind (_relativelocation_x _relativelocation_y _relativelocation_z) (`KismetMathLibrary.BreakVector` (`SceneComponent.RelativeLocation` _staticmesh)))
  (if (`self.Isplay`)
    (if (`self.IsMoveUp`)
      (`SceneComponent.K2_AddRelativeLocation` _staticmesh (`KismetMathLibrary.MakeVector` 0.0 0.0 (* (* DeltaSeconds (`self.Speed`)) -1.0)) false false)
      (if (>= _relativelocation_z 10000.0)
        (set `self.IsMoveUp` false)))))

(fn `MoveDown`
  (params (A :type "Float (double-precision)")))

(fn `UserConstructionScript`)