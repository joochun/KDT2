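; BP_Bullet_2 is a cannon projectile with a gold mesh that damages and ragdolls the player character it hits.
; Each tick it rotates the mesh to face its velocity.
; On any hit, EventHitCharacter adds damage through BP_PlayerState and triggers ragdoll on BP_ThirdPersonCharacter, then DestroyHoming spawns an explosion and destroys the actor.
; Impulse launch, timed self-destruct and player-homing logic are present but disconnected, so they never run.
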(event `self.ReceiveTick`
  (params (DeltaSeconds :type "Float (single-precision)"))
  (bind _sm_gold (`self.SM_Gold`))
  ;[1 1 1] 낙하 방향
  (`SceneComponent.K2_SetWorldRotation` _sm_gold (`KismetMathLibrary.Conv_VectorToRotator` (`SceneComponent.GetComponentVelocity` _sm_gold)) false false))

(event `self.ReceiveBeginPlay`)

(event `self.SM_Gold.OnComponentHit`
  (params (HitComponent :type "PrimitiveComponent Object Reference") (OtherActor :type "Actor Object Reference") (OtherComp :type "PrimitiveComponent Object Reference") (NormalImpulse :type "Vector Structure") (Hit :type "HitResult Structure (by ref)"))
  (`self.EventHitCharacter` OtherActor)
  (`self.DestroyHoming`))

(fn `DestroyHoming`
  (bind _sm_gold (`self.SM_Gold`))
  (`GameplayStatics.SpawnEmitterAtLocation` "/Game/StarterContent/Particles/P_Explosion.P_Explosion" (`SceneComponent.K2_GetComponentLocation` _sm_gold) (`SceneComponent.K2_GetComponentRotation` _sm_gold))
  (`self.K2_DestroyActor`))

(fn `EventHitCharacter`
  (params (Actor :type "Actor Object Reference"))
  (bind _asbp_third_person_character (cast `/Game/ThirdPerson/Blueprints/BP_ThirdPersonCharacter` Actor))
  (bind _asbp_player_state (cast `/Game/CoinGame/GameMode/BP_PlayerState` (`Pawn.PlayerState` _asbp_third_person_character)))
  (`/Game/CoinGame/GameMode/BP_PlayerState.AddDamage` _asbp_player_state 10.0)
  (`/Game/ThirdPerson/Blueprints/BP_ThirdPersonCharacter.DoRagdoll` _asbp_third_person_character))

(fn `UserConstructionScript`)