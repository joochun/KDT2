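; BP_MoveTimeLine is an actor that slides a Cube back and forth along its relative X axis using a timeline scaled by Distance.
; EventPlay and EventStop toggle IsPlay, which Tick checks to run or stop the timeline.
; IsRight selects forward or reverse playback and flips on Finished to create a ping-pong loop.
; Player 0 input is enabled, with debug-style keys to restart, reverse from end or set timeline time.
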(event `self.ReceiveBeginPlay`
  (`self.EnableInput` (`GameplayStatics.GetPlayerController` 0)))

(event `Key|P`
  (params (Key :type "Key Structure")))

(event `self.ReceiveTick`
  (params (DeltaSeconds :type "Float (single-precision)"))
  (if (`self.IsPlay`)
    (if (`self.IsRight`) :!label _label
      (bind (_direction _value) (`Timeline|타임라인` :`NewTime` 0.2 :!label _label_2)
        (:`Update`
          (`SceneComponent.K2_SetRelativeLocation` (`self.Cube`) (`KismetMathLibrary.MakeVector` (* _value (`self.Distance`))) false false))
        (:`Finished`
          (set `self.IsRight` (not (`self.IsRight`)))
          (goto _label)))
      (else
        (goto _label_2 :!via `Reverse`)))
    (else
      (goto _label_2 :!via `Stop`))))

(event `Key|K`
  (params (Key :type "Key Structure"))
  (:`Pressed`
    (goto _label_2 :!via `PlayFromStart`)))

(event `Key|L`
  (params (Key :type "Key Structure"))
  (:`Pressed`
    (goto _label_2 :!via `ReverseFromEnd`)))

(event `Key|O`
  (params (Key :type "Key Structure"))
  (:`Pressed`
    (goto _label_2 :!via `SetNewTime`)))

(event `/Game/Project/BPI_MoveActor.Event Play`
  (set `self.IsPlay` true))

(event `/Game/Project/BPI_MoveActor.Event Stop`
  (set `self.IsPlay` false))

(fn `UserConstructionScript`)