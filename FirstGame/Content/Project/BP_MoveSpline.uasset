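; BP_MoveSpline is an actor that moves a Cube component back and forth along its Spline.
; A timeline value, scaled by spline length, gives the distance used to set the cube's world location.
; When the timeline finishes, IsRight flips to switch between Play and Reverse.
; EventPlay and EventStop toggle IsPlay, which Tick checks every frame to drive or stop the timeline.
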(event `self.ReceiveBeginPlay`)

(event `self.ReceiveTick`
  (params (DeltaSeconds :type "Float (single-precision)"))
  (if (`self.IsPlay`)
    (if (`self.IsRight`) :!label _label
      (bind (_direction _value) (`Timeline|타임라인` :`NewTime` 0.5 :!label _label_2)
        (:`Update`
          (`SceneComponent.K2_SetWorldLocation` (`self.Cube`) (`SplineComponent.GetLocationAtDistanceAlongSpline` (`self.Spline`) (* _value (`SplineComponent.GetSplineLength` (`self.Spline`))) "World") false false))
        (:`Finished`
          (set `self.IsRight` (not (`self.IsRight`)))
          (goto _label)))
      (else
        (goto _label_2 :!via `Reverse`)))
    (else
      (goto _label_2 :!via `Stop`))))

(event `/Game/Project/BPI_MoveActor.Event Play`
  (set `self.IsPlay` true))

(event `/Game/Project/BPI_MoveActor.Event Stop`
  (set `self.IsPlay` false))

(fn `UserConstructionScript`)