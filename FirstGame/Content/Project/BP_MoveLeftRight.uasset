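; BP_MoveLeftRight is an actor that slides its Sphere component back and forth along its relative X axis.
; While IsPlay is set, Tick moves the sphere by Speed scaled with delta time, flipping IsMoveRight when it reaches the fixed bounds at either end.
; EventPlay and EventStop set and clear IsPlay to start and pause the motion.
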(event `self.ReceiveTick`
  (params (DeltaSeconds :type "Float (single-precision)"))
  (bind _sphere (`self.Sphere`))
  (bind _sphere_2 (`self.Sphere`))
  (bind _returnvalue (* DeltaSeconds (`self.Speed`)))
  (bind _relativelocation_x (`KismetMathLibrary.BreakVector` (`SceneComponent.RelativeLocation` _sphere)))
  (bind _relativelocation_x_2 (`KismetMathLibrary.BreakVector` (`SceneComponent.RelativeLocation` _sphere_2)))
  (if (`self.IsPlay`)
    (if (`self.IsMoveRight`)
      (`SceneComponent.K2_AddRelativeLocation` _sphere (`KismetMathLibrary.MakeVector` _returnvalue) false false)
      (if (>= _relativelocation_x 500.0)
        (set `self.IsMoveRight` false))
      (else
        (`SceneComponent.K2_AddRelativeLocation` _sphere_2 (`KismetMathLibrary.MakeVector` (* _returnvalue -1.0)) false false)
        (if (<= _relativelocation_x_2 0.0)
          (set `self.IsMoveRight` true))))))

(event `/Game/Project/BPI_MoveActor.Event Play`
  (set `self.IsPlay` true))

(event `/Game/Project/BPI_MoveActor.Event Stop`
  (set `self.IsPlay` false))

(fn `UserConstructionScript`)